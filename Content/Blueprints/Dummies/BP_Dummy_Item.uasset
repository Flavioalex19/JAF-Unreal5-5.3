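; BP_Dummy_Item is a placeholder item actor with a Cube component that starts hidden in game and always reports that it cannot be interacted with.
; The IsVisible event shows the cube with physics-only collision when active, or hides it and disables collision otherwise.
; BeginPlay only hides the cube, leaving its collision setting untouched until IsVisible is called.
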(event EventBeginPlay
  (Development|SetHiddeninGame (Variables|Default|GetCube) true false))

(event Collision|EventActorBeginOverlap
  (params (OtherActor :type Actor%20Object%20Reference)))

(event EventTick
  (params (DeltaSeconds :type Float%20%28single-precision%29)))

(event EventIsVisible
  (params (Is%20active :type Boolean))
  (if Is%20active
    (Development|SetHiddeninGame (Variables|Default|GetCube) false false)
    (Collision|SetCollisionEnabled (Variables|Default|GetCube) "PhysicsOnly")
    (else
      (Development|SetHiddeninGame (Variables|Default|GetCube) true false)
      (Collision|SetCollisionEnabled (Variables|Default|GetCube) "NoCollision"))))

(fn ConstructionScript)

(fn CanInteract?
  (return false))