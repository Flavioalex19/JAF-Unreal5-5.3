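; BP_GameManager manages the dialogue UI, creating a Widget_Dialogue on BeginPlay and adding it to the viewport.
; DialogueTextUpdate sets the widget's text, while UIDialoguePanelUpdate and DialogueEndConversation switch the panel flag on and off.
; Tick polls that flag, playing the open animation once through a DoOnce that resets on conversation end.
; While closed, it replays the close animation and sets placeholder text every frame.
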(event EventUIDialoguePanelUpdate
  (params (Is%20On :type Boolean))
  ;[1 1 1] Update Dialogue Text
  (if (not (Variables|Default|GetIs%20Dialogue%20Panel%20On))
    (Variables|Default|SetIs%20Dialogue%20Panel%20On true)))

(event EventDialogueTextUpdate
  (params (Dialogue%20Text :type String) (Dialogue%20Index :type Integer))
  (Rendering|Components|TextRender|SetText (Variables|/Game/UI/Widget_Dialogue.Widget_Dialogue_C|GetDialoguetext (stale EventBeginPlay _returnvalue)) (Utilities|Text|ToText(String) Dialogue%20Text)))

(event EventDialogueEndConversation
  (params (Is%20on :type Boolean))
  ;[1 1 1] Update Dialogue Text
  (Variables|Default|SetIs%20Dialogue%20Panel%20On false)
  (Development|PrintString "reset")
  (Utilities|FlowControl|DoOnce false) ; enters at Reset
)

(event EventBeginPlay
  ;[1 1 1] Update Dialogue Text
  (bind _returnvalue (UserInterface|CreateWidget "/Game/UI/Widget_Dialogue.Widget_Dialogue_C"))
  (UserInterface|Viewport|AddtoViewport _returnvalue 0))

(event EventUIUpdate
  (params (Is%20On :type Boolean) (Dialogue%20Text :type String)))

(event EventTick
  (params (DeltaSeconds :type Float%20%28single-precision%29))
  ;[1 1 1] Update Dialogue Text
  (if (Variables|Default|GetIs%20Dialogue%20Panel%20On)
    (Utilities|FlowControl|DoOnce false
      (:Completed
        (UserInterface|Animation|PlayAnimation (stale EventBeginPlay _returnvalue) (Variables|/Game/UI/Widget_Dialogue.Widget_Dialogue_C|GetDialogue_Panel_On (stale EventBeginPlay _returnvalue)) 0.0 1 "Forward" 1.0 false)))
    (else
      (UserInterface|Animation|PlayAnimation (stale EventBeginPlay _returnvalue) (Variables|/Game/UI/Widget_Dialogue.Widget_Dialogue_C|GetDialogue_Panel_Off (stale EventBeginPlay _returnvalue)) 0.0 1 "Forward" 1.0 false)
      (Rendering|Components|TextRender|SetText (Variables|/Game/UI/Widget_Dialogue.Widget_Dialogue_C|GetDialoguetext (stale EventBeginPlay _returnvalue)) "lol"))))

(fn ConstructionScript)