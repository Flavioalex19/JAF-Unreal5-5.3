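; BP_Point is a two-way warp waypoint that teleports the player pawn between capsules A and B.
; Overlapping either capsule enables activation and selects the opposite capsule as destination, without filtering the overlapping actor, and leaving disables it.
; The Warping event, which nothing in this graph calls, performs the teleport when enabled and resets the pawn's rotation to zero.
; CanInteract always returns false.
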(event OnComponentBeginOverlap(TP_CapsuleA)
  (params (OverlappedComponent :type Primitive%20Component%20Object%20Reference) (OtherActor :type Actor%20Object%20Reference) (OtherComp :type Primitive%20Component%20Object%20Reference) (OtherBodyIndex :type Integer) (bFromSweep :type Boolean) (SweepResult :type Hit%20Result%20Structure%20%28by%20ref%29))
  ;[1 1 1] Warp point A to point B
  (Variables|Default|SetCan%20Activate true)
  (Variables|Default|SetIs_TP_A? false))

(event OnComponentBeginOverlap(TP_CapsuleB)
  (params (OverlappedComponent :type Primitive%20Component%20Object%20Reference) (OtherActor :type Actor%20Object%20Reference) (OtherComp :type Primitive%20Component%20Object%20Reference) (OtherBodyIndex :type Integer) (bFromSweep :type Boolean) (SweepResult :type Hit%20Result%20Structure%20%28by%20ref%29))
  ;[1 1 1] Warp point A to point B
  (Variables|Default|SetCan%20Activate true)
  (Variables|Default|SetIs_TP_A? true))

(event OnComponentEndOverlap(TP_CapsuleA)
  (params (OverlappedComponent :type Primitive%20Component%20Object%20Reference) (OtherActor :type Actor%20Object%20Reference) (OtherComp :type Primitive%20Component%20Object%20Reference) (OtherBodyIndex :type Integer))
  ;[1 1 1] Warp point A to point B
  (Variables|Default|SetCan%20Activate false))

(event OnComponentEndOverlap(TP_CapsuleB)
  (params (OverlappedComponent :type Primitive%20Component%20Object%20Reference) (OtherActor :type Actor%20Object%20Reference) (OtherComp :type Primitive%20Component%20Object%20Reference) (OtherBodyIndex :type Integer))
  ;[1 1 1] Warp point A to point B
  (Variables|Default|SetCan%20Activate false))

(event EventWarping
  (params (Can%20TP_A :type Boolean))
  ;[1 1 1] Warp point A to point B
  (if (Variables|Default|GetCan%20Activate)
    (if (Variables|Default|GetIs_TP_A?)
      (Transformation|Teleport (Game|Player|GetPlayerPawn 0) (Transformation|GetWorldLocation (Variables|Default|GetTP_CapsuleA)) "0, 0, 0")
      (else
        (Transformation|Teleport (Game|Player|GetPlayerPawn 0) (Transformation|GetWorldLocation (Variables|Default|GetTP_CapsuleB)) "0, 0, 0")))))

(fn ConstructionScript)

(fn CanInteract?
  (return false))