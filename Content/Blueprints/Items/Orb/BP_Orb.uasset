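; BP_Orb is an interactable orb item whose point light toggles between green and white.
; On ObjInteraction, if the player pawn overlaps its Sphere, a FlipFlop switches the light color, sets IsEnlightened and prints On or Off.
; CanInteract always returns false, and ending the sphere overlap only clears IsIn.
; Gate and input enable/disable nodes are left unconnected.
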(event OnComponentEndOverlap(Sphere)
  (params (OverlappedComponent :type Primitive%20Component%20Object%20Reference) (OtherActor :type Actor%20Object%20Reference) (OtherComp :type Primitive%20Component%20Object%20Reference) (OtherBodyIndex :type Integer))
  (Variables|Default|SetIs%20in false))

(event EventObjInteraction
  (if (Collision|IsOverlappingActor (Variables|Default|GetSphere) (Game|Player|GetPlayerPawn 0) :!class /Script/Engine.PrimitiveComponent)
    (Utilities|FlowControl|FlipFlop
      (:A
        (Rendering|Components|Light|SetLightColor (Variables|Default|GetPointLight) "(R=0.044338,G=0.291667,B=0.000000,A=1.000000)" true)
        (Variables|Default|SetIs%20Enlightened true)
        (Development|PrintString "On"))
      (:B
        (Rendering|Components|Light|SetLightColor (Variables|Default|GetPointLight) "(R=1.000000,G=1.000000,B=1.000000,A=1.000000)" true)
        (Variables|Default|SetIs%20Enlightened false)
        (Development|PrintString "Off")))))

(fn ConstructionScript)

(fn CanInteract?
  (return false))