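; BP_Item is a test item actor that removes itself when interacted with while a main character overlaps it.
; ItemInteraction searches overlapping BP_MainCharacter actors and destroys the item at the first one implementing BPI_Interaction, without passing any item data to it.
; BeginPlay writes the BP_Item class into a freshly made STRItems struct of placeholder values, which is not stored in a variable.
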(event EventItemInteraction
  ;[1 1 1] Item Interaction BP
  (bind _array_element (Utilities|Array|ForEachLoopwithBreak (Collision|GetOverlappingActors "/Game/Blueprints/BP_MainCharacter.BP_MainCharacter_C" :!class /Script/Engine.Actor) :!label _label)
    (:LoopBody
      (if (Utilities|DoesObjectImplementInterface _array_element "/Game/Blueprints/Interfaces/BPI_Interaction.BPI_Interaction_C")
        (Actor|DestroyActor)
        (goto _label Break)))))

(event EventBeginPlay
  ;[1 1 1] Set Class on Structure as BP_Item Class
  (|SetBy-RefVar (.Class (Utilities|Struct|BreakSTR_Items (Utilities|Struct|MakeSTR_Items "None" 0 "Test Item" false "None" "BP_Item_C"))) "BP_Item_C"))

(fn ConstructionScript
  (|CallParentFunction))