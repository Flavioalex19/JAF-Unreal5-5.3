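; Main character Blueprint handling interaction, damage and a partly built absorb skill.
; Flashlight input, gated by DoOnce until release, sends BPI_Interaction messages to overlapping warp points and orbs; interaction input does so for items.
; Damage lowers HP unless CanAbsorb is set.
; While the skill enabler is held, Absorb activates the skill and clears CanBeHit; Tick counts its timer down but only prints at exactly zero.
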(event Input|EnhancedActionEvents|EnhancedInputActionIA_Flashlight
  (params (ActionValue :type Boolean) (ElapsedSeconds :type Float%20%28double-precision%29) (TriggeredSeconds :type Float%20%28double-precision%29) (InputAction :type Input%20Action%20Object%20Reference :default "/Game/Inputs/IA_Flashlight.IA_Flashlight"))
  ;[1 1 1] Flashlight Function
  (:Triggered
    (Utilities|FlowControl|DoOnce false :!label _label
      (:Completed
        (bind _array_element (Utilities|Array|ForEachLoopwithBreak (Collision|GetOverlappingActors (Variables|Default|GetCapsuleComponent) "/Game/Blueprints/Items/Orb/BP_Orb.BP_Orb_C" :!class /Script/Engine.PrimitiveComponent) :!label _label_2)
          (:LoopBody
            (if (Utilities|DoesObjectImplementInterface _array_element "/Game/Blueprints/Interfaces/BPI_Interaction.BPI_Interaction_C")
              (Class|BPIInteraction|ObjInteraction(Message) _array_element)
              (goto _label_2 Break)))))))
  (:Completed
    (goto _label Reset)))

(event Input|EnhancedActionEvents|EnhancedInputActionIA_Skill_Enabler
  (params (ActionValue :type Boolean) (ElapsedSeconds :type Float%20%28double-precision%29) (TriggeredSeconds :type Float%20%28double-precision%29) (InputAction :type Input%20Action%20Object%20Reference :default "/Game/Inputs/IA_Skill_Enabler.IA_Skill_Enabler"))
  ;[1 1 1] Skill Enabler
  (:Triggered
    (Variables|Default|SetIs%20Skill%20Enabled? ActionValue :!label _label))
  (:Ongoing
    (goto _label))
  (:Canceled
    (Variables|Default|SetIs%20Skill%20Enabled? false :!label _label_2))
  (:Completed
    (goto _label_2)))

(event Input|EnhancedActionEvents|EnhancedInputActionIA_Flashlight
  (params (ActionValue :type Boolean) (ElapsedSeconds :type Float%20%28double-precision%29) (TriggeredSeconds :type Float%20%28double-precision%29) (InputAction :type Input%20Action%20Object%20Reference :default "/Game/Inputs/IA_Flashlight.IA_Flashlight"))
  ;[1 1 1] Warp function (change to IA Interaction later)
  (:Triggered
    (Utilities|FlowControl|DoOnce false :!label _label
      (:Completed
        (bind _array_element (Utilities|Array|ForEachLoopwithBreak (Collision|GetOverlappingActors (Variables|Default|GetCapsuleComponent) "/Game/Blueprints/Warp_Waypoint/BP_Point.BP_Point_C" :!class /Script/Engine.PrimitiveComponent) :!label _label_2)
          (:LoopBody
            (if (Utilities|DoesObjectImplementInterface _array_element "/Game/Blueprints/Interfaces/BPI_Interaction.BPI_Interaction_C")
              (Class|BPIInteraction|Warping(Message) _array_element false)
              (goto _label_2 Break)))))))
  (:Completed
    (goto _label Reset)))

(event Input|EnhancedActionEvents|EnhancedInputActionIA_Absorb
  (params (ActionValue :type Boolean) (ElapsedSeconds :type Float%20%28double-precision%29) (TriggeredSeconds :type Float%20%28double-precision%29) (InputAction :type Input%20Action%20Object%20Reference :default "/Game/Inputs/IA_Absorb.IA_Absorb"))
  (if (Variables|Default|GetIs%20Skill%20Enabled?)
    (Variables|Default|SetIs%20Skill%20Active true)
    (Variables|Default|SetCanBeHit false)))

(event Input|EnhancedActionEvents|EnhancedInputActionIA_Interaction
  (params (ActionValue :type Boolean) (ElapsedSeconds :type Float%20%28double-precision%29) (TriggeredSeconds :type Float%20%28double-precision%29) (InputAction :type Input%20Action%20Object%20Reference :default "/Game/Inputs/IA_Interaction.IA_Interaction"))
  ;[1 1 1] Item interaction check
  (bind _array_element (Utilities|Array|ForEachLoopwithBreak (Collision|GetOverlappingActors "/Game/Blueprints/Items/BP_Interactable.BP_Interactable_C" :!class /Script/Engine.Actor) :!label _label)
    (:LoopBody
      (if (Utilities|DoesObjectImplementInterface _array_element "/Game/Blueprints/Interfaces/BPI_Interaction.BPI_Interaction_C")
        (Class|BPIInteraction|ItemInteraction(Message) _array_element)
        (goto _label Break)))))

(event EventBeginPlay)

(event EventDamage
  (params (DamageDealt :type Integer))
  ;[1 1 1] Damage
  (if (not (Variables|Default|Getcan%20absorb))
    (Variables|Default|SetHP (- (Variables|Default|GetHP) DamageDealt))))

(event EventTick
  (params (DeltaSeconds :type Float%20%28single-precision%29))
  ;[1 1 1] Timer Reset
  (if (Variables|Default|GetIs%20Skill%20Active)
    (Variables|Default|SetTimer (- (Variables|Default|GetTimer) DeltaSeconds))
    (if (== (Variables|Default|GetTimer) 0.0)
      (Development|PrintString "Time Resetted"))))

(fn ConstructionScript)