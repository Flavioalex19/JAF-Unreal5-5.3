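; BP_NPC_Test is a test NPC that steps through an array of dialogue lines each time Talk is called.
; Talk increments an index, sets a talking flag, and sends the current line to the first BP_GameManager implementing BPI_NPC_Interaction through UIUpdateMessage.
; Past the last line it resets the index and clears the flag without sending a UI update.
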(event EventTalk
  (Math|Integer|IncrementInt (Variables|Default|GetTalkIndex)
    (:%20%20
      (if (< (Variables|Default|GetTalkIndex) (Utilities|Array|Length (Variables|Default|GetDialogue%20Array)))
        (bind _output_get (Variables|Default|SetIs%20Talking true))
        (bind _outactors (Actor|GetAllActorsOfClass "/Game/Blueprints/Managers/BP_GameManager.BP_GameManager_C"))
        (bind _array_element (Utilities|Array|ForEachLoopwithBreak _outactors :!label _label)
          (:LoopBody
            (if (Utilities|DoesObjectImplementInterface _array_element "/Game/Blueprints/Interfaces/BPI_NPC_Interaction.BPI_NPC_Interaction_C")
              (Class|BPINPCInteraction|UIUpdate(Message) _array_element _output_get (Utilities|Array|Get(acopy) (Variables|Default|GetDialogue%20Array) (Variables|Default|GetTalkIndex)))
              (goto _label Break))))
        (else
          (Variables|Default|SetTalkIndex -1)
          (Variables|Default|SetIs%20Talking false))))))

(fn ConstructionScript)